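; NukeBP is a bomb actor with a physics-driven Box that produces an explosion effect and removes itself.
; Each Tick checks the Box's Z velocity and, once it turns positive, switches off physics simulation and prints a debug name.
; After a short delay it spawns a scaled-up P_Explosion emitter at the Box's location, prints a message and destroys the actor, applying no damage.
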(event EventTick
  (params (DeltaSeconds :type Float%20%28single-precision%29))
  (bind _returnvalue (Physics|GetPhysicsLinearVelocity (Variables|Default|GetBox) "None"))
  (if (> (.z _returnvalue) 0.0)
    (Physics|SetSimulatePhysics (Variables|Default|GetBox) false)
    (Development|PrintString (Utilities|GetDisplayName 0))
    (Utilities|FlowControl|Delay 1.5)
    (Effects|SpawnEmitteratLocation "/Game/StarterContent/Particles/P_Explosion.P_Explosion" (Transformation|GetWorldLocation (Variables|Default|GetBox)) "0, 0, 0" "10.000000,10.000000,10.000000")
    (Development|PrintString "EXPLOTAAAAA")
    (Actor|DestroyActor)))

(fn ConstructionScript)