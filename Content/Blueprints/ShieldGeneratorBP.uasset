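; Shield generator actor, apparently a stratagem drop, that deploys a Shield once it lands.
; Each tick while its Box simulates physics, an upward Z velocity is treated as the bounce off the floor and switches physics off, which also stops the check repeating.
; It then plays a touchdown sound, waits briefly, spawns the Shield at the generator's location and plays the shield sound.
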(event EventTick
  (params (DeltaSeconds :type Float%20%28single-precision%29))
  (bind _box (Variables|Default|GetBox))
  (if (Physics|IsSimulatingPhysics _box "None")
    (bind _returnvalue (Physics|GetPhysicsLinearVelocity _box "None"))
    (if (> (.z _returnvalue) 0.0)
      (Physics|SetSimulatePhysics (Variables|Default|GetBox) false)
      (Audio|PlaySound2D "/Game/Audio/StratagemTouchFloorQue.StratagemTouchFloorQue" 1.0 1.0 0.0 0 0)
      (Utilities|FlowControl|Delay 1.5)
      (Game|SpawnActorfromClass "/Game/Blueprints/Shield.Shield_C" (Math|Conversions|ToTransform(Vector) (Transformation|GetWorldLocation (Variables|Default|GetShieldGenerator))) "Undefined" "MultiplyWithRoot" 0 0)
      (Audio|PlaySound2D "/Game/Audio/ShieldCue.ShieldCue" 1.0 1.0 0.0 0 0))))

(fn ConstructionScript)